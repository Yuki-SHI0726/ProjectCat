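; BP_Gimmick is a level gimmick actor, apparently a base, that reacts to bullets and the player entering its capsule.
; Overlapping actors tagged Bullet are cast to BP_Bullet_RPS and passed to HitByBullet, which is an empty stub.
; A player character overlap fires the gimmick action through a DoOnce, reset when the player leaves.
; The gimmick action itself only prints a placeholder message.
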(event `self.Capsule.OnComponentBeginOverlap`
  (params (OverlappedComponent :type "PrimitiveComponent Object Reference") (OtherActor :type "Actor Object Reference") (OtherComp :type "PrimitiveComponent Object Reference") (OtherBodyIndex :type Integer) (bFromSweep :type Boolean) (SweepResult :type "HitResult Structure (by ref)"))
  (if (`self.ActorHasTag` OtherActor "Bullet")
    (bind _asbp_bullet_rps (cast `/Game/ProjectCat/Actors/BulletBP/BP_Bullet_RPS` OtherActor))
    (`self.HitByBullet` _asbp_bullet_rps)
    (else
      (cast `/Game/ProjectCat/Characters/Player/BP_PlayerCharacter` OtherActor)
      (`/Engine/EditorBlueprintResources/StandardMacros.DoOnce` false :!label _label
        (:`Completed`
          (`self.CE_GimmickAction`))))))

(event `self.Capsule.OnComponentEndOverlap`
  (params (OverlappedComponent :type "PrimitiveComponent Object Reference") (OtherActor :type "Actor Object Reference") (OtherComp :type "PrimitiveComponent Object Reference") (OtherBodyIndex :type Integer))
  (cast `/Game/ProjectCat/Characters/Player/BP_PlayerCharacter` OtherActor)
  (goto _label :!via `Reset`))

(event `CE_GimmickAction`
  (`KismetSystemLibrary.PrintString` "Gimmick Working!"))

(fn `HitByBullet`
  (params (HitBullet :type "/Game/ProjectCat/Actors/BulletBP/BP_Bullet_RPS Object Reference")))

(fn `UserConstructionScript`)
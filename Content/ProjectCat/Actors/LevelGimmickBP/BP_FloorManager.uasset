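; Floor manager actor that builds a rows-by-columns grid of BP_Floor tiles extending from its own location.
; CE_SpawnAllFloor destroys the tiles tracked in FloorList, then spawns each new tile with its size and sequential number and adds it to the list.
; CalcFloorLocation spaces tiles at twice the floor length along X and Y.
; Nothing here calls the spawn event, and FloorList is never emptied after destruction.
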(event `CE_SpawnAllFloor`
  (bind _rownumber (`self.RowNumber`))
  (`self.DestroyAllCurrentFloors`)
  (for _index (range 1 (+ (`self.ColNumber`) 1))
    (for _index_2 (range 1 (+ _rownumber 1))
      (bind _outlocation (`self.CalcFloorLocation` _index_2 _index))
      (bind _returnvalue (`|SpawnActorFromClass` "/Game/ProjectCat/Actors/LevelGimmickBP/BP_Floor.BP_Floor_C" (`KismetMathLibrary.MakeTransform` _outlocation) "Undefined" "OverrideRootScale" null (`self.FloorRecLength`) (`self.FloorRecHeight`) (+ _index_2 (* (- _index 1) _rownumber)) null))
      (`KismetArrayLibrary.Array_Add` (`self.FloorList`) _returnvalue))))

(fn `CalcFloorLocation`
  (params (CurrentRow :type Integer) (CurrentCol :type Integer))
  (returns (OutLocation :type "Vector Structure"))
  (locals (LocationOut :type "Vector Structure"))
  (bind (_returnvalue_x _returnvalue_y _returnvalue_z) (`KismetMathLibrary.BreakVector` (`self.K2_GetActorLocation`)))
  (bind _output_get (set `local.LocationOut` (`KismetMathLibrary.MakeVector` (+ (`KismetMathLibrary.Conv_IntToDouble` (* (- CurrentRow 1) (* (`self.FloorRecLength`) 2))) _returnvalue_x) (+ (`KismetMathLibrary.Conv_IntToDouble` (* (- CurrentCol 1) (* (`self.FloorRecLength`) 2))) _returnvalue_y) _returnvalue_z)))
  (return _output_get))

(fn `DestroyAllCurrentFloors`
  (bind (_arrayindex _arrayelement) (`/Engine/EditorBlueprintResources/StandardMacros.ReverseForEachLoop` (`self.FloorList`))
    (:`LoopBody`
      (`self.K2_DestroyActor` _arrayelement))
    (:`Completed`
      (`KismetSystemLibrary.PrintString` "All Floor Cleared!"))))

(fn `UserConstructionScript`
  (locals (ColCount :type Integer) (RowCount :type Integer)))
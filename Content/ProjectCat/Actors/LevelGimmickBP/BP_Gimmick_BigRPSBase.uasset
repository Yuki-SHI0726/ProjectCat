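; Base rock-paper-scissors target gimmick that bullets can hit to score points for their caster.
; Activation makes it targetable after a short delay; a valid hit compares bullet and target types, awards points only for bullet wins, then deactivates it.
; RPSResult inverts wins and losses when NormalPattern is off, which events can randomize or toggle.
; The state randomizer currently yields Rock on every branch, and the construction script displays the state as text.
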(event `CE_OnActivate`
  ;[1 1 1] 台座上升，不可被攻击
  (set `self.CanBeTarget` false)
  (`KismetSystemLibrary.Delay` 0.2)
  (set `self.CanBeTarget` true))

(event `CE_OnDeactivate`
  ;[1 1 1] 台座下降
  (set `self.CanBeTarget` false))

(event `CE_RandomStateRPS`
  ;[1 1 1] 随机决定自身拳头剪刀布
  (switch `int` (`KismetMathLibrary.RandomIntegerInRange` 0 2)
    (:`0`
      (set `self.RPSState` "NewEnumerator0"))
    (:`1`
      (set `self.RPSState` "NewEnumerator0"))
    (:`2`
      (set `self.RPSState` "NewEnumerator0"))))

(event `CE_RandomNormalPattern`
  ;[1 1 1] 随机使用正常石头剪刀布判定规律
  (switch `int` (`KismetMathLibrary.RandomIntegerInRange` 0 1)
    (:`Default`
      (set `self.NormalPattern` true :!label _label))
    (:`0`
      (set `self.NormalPattern` false))
    (:`1`
      (goto _label))))

(event `CE_ChangePattern`
  ;[1 1 1] 改变石头剪刀布正负判定规律
  (if (`self.NormalPattern`)
    (set `self.NormalPattern` false)
    (else
      (set `self.NormalPattern` true))))

(fn `HitByBullet`
  (params (HitBullet :type "/Game/ProjectCat/Actors/BulletBP/BP_Bullet_RPS Object Reference"))
  (bind _caster (`/Game/ProjectCat/Actors/BulletBP/BP_Bullet_RPS.Caster` HitBullet))
  (if (`self.CanBeTarget`)
    (bind _finalresult (`self.RPSResult` (`/Game/ProjectCat/Actors/BulletBP/BP_Bullet_RPS.RockPaperScissor` HitBullet) (`self.RPSState`) (`self.NormalPattern`)))
    (switch `/Game/ProjectCat/Actors/BulletBP/Enum_RockPaperScissorResult` _finalresult
      (:`NewEnumerator0`
        (`/Game/ProjectCat/Characters/Player/BP_PlayerCharacter.Add Score` _caster 2 "NewEnumerator0"))
      (:`NewEnumerator1`
        (`/Game/ProjectCat/Characters/Player/BP_PlayerCharacter.Add Score` _caster 0 "NewEnumerator1"))
      (:`NewEnumerator2`
        (`/Game/ProjectCat/Characters/Player/BP_PlayerCharacter.Add Score` _caster 0 "NewEnumerator2")))
    (`self.CE_OnDeactivate`)))

(fn `RPSResult`
  (params (FirstType :type "/Game/ProjectCat/Actors/BulletBP/Enum_RockPaperScissor Enum" :default "NewEnumerator0") (SecondType :type "/Game/ProjectCat/Actors/BulletBP/Enum_RockPaperScissor Enum" :default "NewEnumerator0") (NormalPattern :type Boolean))
  (returns (FinalResult :type "/Game/ProjectCat/Actors/BulletBP/Enum_RockPaperScissorResult Enum"))
  (locals (SecondTypeLocal :type "/Game/ProjectCat/Actors/BulletBP/Enum_RockPaperScissor Enum" :default "NewEnumerator0") (RPSBulletWinNormalPattern :type Boolean) (NormalResult :type "/Game/ProjectCat/Actors/BulletBP/Enum_RockPaperScissorResult Enum") (IsNormalPattern :type Boolean))
  (set `local.IsNormalPattern` NormalPattern)
  (set `local.SecondTypeLocal` SecondType)
  (switch `/Game/ProjectCat/Actors/BulletBP/Enum_RockPaperScissor` FirstType
    (:`NewEnumerator0`
      (switch `/Game/ProjectCat/Actors/BulletBP/Enum_RockPaperScissor` (`local.SecondTypeLocal`)
        (:`NewEnumerator0`
          (set `local.NormalResult` "NewEnumerator1"))
        (:`NewEnumerator1`
          (set `local.NormalResult` "NewEnumerator2"))
        (:`NewEnumerator2`
          (set `local.NormalResult` "NewEnumerator0"))))
    (:`NewEnumerator1`
      (switch `/Game/ProjectCat/Actors/BulletBP/Enum_RockPaperScissor` (`local.SecondTypeLocal`)
        (:`NewEnumerator0`
          (set `local.NormalResult` "NewEnumerator0"))
        (:`NewEnumerator1`
          (set `local.NormalResult` "NewEnumerator1"))
        (:`NewEnumerator2`
          (set `local.NormalResult` "NewEnumerator2"))))
    (:`NewEnumerator2`
      (switch `/Game/ProjectCat/Actors/BulletBP/Enum_RockPaperScissor` (`local.SecondTypeLocal`)
        (:`NewEnumerator0`
          (set `local.NormalResult` "NewEnumerator2"))
        (:`NewEnumerator1`
          (set `local.NormalResult` "NewEnumerator0"))
        (:`NewEnumerator2`
          (set `local.NormalResult` "NewEnumerator1")))))
  (if (`self.NormalPattern`)
    (return (`local.NormalResult`))
    (else
      (switch `/Game/ProjectCat/Actors/BulletBP/Enum_RockPaperScissorResult` (`local.NormalResult`)
        (:`NewEnumerator0`
          (return "NewEnumerator2"))
        (:`NewEnumerator1`
          (return "NewEnumerator1"))
        (:`NewEnumerator2`
          (return "NewEnumerator0"))))))

(fn `UserConstructionScript`
  (`parent.UserConstructionScript`)
  (`TextRenderComponent.K2_SetText` (`self.RPSStaterenderer`) (`KismetTextLibrary.Conv_StringToText` (`|GetEnumeratorNameAsString` (`self.RPSState`)))))
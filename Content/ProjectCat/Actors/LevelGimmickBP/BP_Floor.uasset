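; Floor tile level gimmick that can turn into a falling trap for the player.
; CE_FloorTrapActivate sets trap mode and plays a timeline that lowers the actor along Z by FallDistance, arming tripping as it moves.
; Once armed, players who begin overlapping the Box receive CEStepOnTrap.
; The construction script scales the mesh uniformly from FloorRectLength and sizes the Box from that length and FloorRectHeight.
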(event `CE_FloorTrapActivate`
  (bind (_actorlocation_x _actorlocation_y _actorlocation_z) (`KismetMathLibrary.BreakVector` (`self.ActorLocation`)))
  ;[1 1 1] 地板陷落
  (set `self.IsTrapMode` true)
  (set `self.ActorLocation` (`self.K2_GetActorLocation`))
  (bind (_direction _newtrack_0) (`Timeline|Timeline_0` :`NewTime` (`GameplayStatics.GetWorldDeltaSeconds`))
    (:`Update`
      (`self.K2_SetActorLocation` (`KismetMathLibrary.MakeVector` _actorlocation_x _actorlocation_y (- _actorlocation_z (* _newtrack_0 (`self.FallDistance`)))))
      (set `self.StartTripping` true))))

(event `self.Box.OnComponentBeginOverlap`
  (params (OverlappedComponent :type "PrimitiveComponent Object Reference") (OtherActor :type "Actor Object Reference") (OtherComp :type "PrimitiveComponent Object Reference") (OtherBodyIndex :type Integer) (bFromSweep :type Boolean) (SweepResult :type "HitResult Structure (by ref)"))
  (if (`self.StartTripping`)
    (bind _asbp_player_character (cast `/Game/ProjectCat/Characters/Player/BP_PlayerCharacter` OtherActor))
    (`/Game/ProjectCat/Characters/Player/BP_PlayerCharacter.CE_StepOnTrap` _asbp_player_character)))

(fn `UserConstructionScript`
  (bind _floorrectlength (`self.FloorRectLength`))
  (bind _returnvalue (/ (`KismetMathLibrary.Conv_IntToDouble` (`self.FloorRectLength`)) 65.0))
  (`SceneComponent.SetWorldScale3D` (`self.StaticMesh`) (`KismetMathLibrary.MakeVector` _returnvalue _returnvalue _returnvalue))
  (`BoxComponent.SetBoxExtent` (`self.Box`) (`KismetMathLibrary.MakeVector` (`KismetMathLibrary.Conv_IntToDouble` _floorrectlength) (`KismetMathLibrary.Conv_IntToDouble` _floorrectlength) (`KismetMathLibrary.Conv_IntToDouble` (`self.FloorRectHeight`))) true))
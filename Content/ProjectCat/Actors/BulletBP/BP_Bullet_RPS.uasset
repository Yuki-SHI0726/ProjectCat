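; Bullet actor that carries a rock-paper-scissors type and shows it as a text label turned to face the camera every tick.
; On BeginPlay it writes the enum to the label and switches on the type, though no case has logic attached.
; Overlaps with owners not tagged Bullet or Player spawn an effect and destroy it after a brief delay.
; Hits add a sound and destroy it immediately; construction sets its lifespan.
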(event `self.ReceiveBeginPlay`
  (`self.CE_ChangeShape`))

(event `CE_ChangeShape`
  (`|ExecutionSequence`
    (:`then_0`
      (`self.CE_TextDisplay`))
    (:`then_1`
      (switch `/Game/ProjectCat/Actors/BulletBP/Enum_RockPaperScissor` (`self.RockPaperScissor`)))))

(event `CE_TextDisplay`
  (`TextRenderComponent.K2_SetText` (`self.TextRender`) (`KismetTextLibrary.Conv_StringToText` (`|GetEnumeratorNameAsString` (`self.RockPaperScissor`)))))

(event `CE_TextToCamera`
  (`SceneComponent.K2_SetWorldRotation` (`self.TextRender`) (`KismetMathLibrary.Conv_VectorToRotator` (- (`self.CameraLocation`) (`self.K2_GetActorLocation`))) false false))

(event `self.ReceiveTick`
  (params (DeltaSeconds :type "Float (single-precision)"))
  (`self.CE_TextToCamera`))

(event `self.Sphere.OnComponentBeginOverlap`
  (params (OverlappedComponent :type "PrimitiveComponent Object Reference") (OtherActor :type "Actor Object Reference") (OtherComp :type "PrimitiveComponent Object Reference") (OtherBodyIndex :type Integer) (bFromSweep :type Boolean) (SweepResult :type "HitResult Structure (by ref)"))
  (bind _returnvalue (`ActorComponent.GetOwner` OtherComp))
  (if (`self.ActorHasTag` _returnvalue "Bullet")
    _
    (elif (not (`self.ActorHasTag` _returnvalue "Player"))
      (`NiagaraFunctionLibrary.SpawnSystemAtLocation` null (`self.K2_GetActorLocation`))
      (`PrimitiveComponent.SetCollisionEnabled` (`self.Sphere`) "NoCollision")
      (`KismetSystemLibrary.Delay` 0.1)
      (`self.K2_DestroyActor`))))

(event `self.Sphere.OnComponentHit`
  (params (HitComponent :type "PrimitiveComponent Object Reference") (OtherActor :type "Actor Object Reference") (OtherComp :type "PrimitiveComponent Object Reference") (NormalImpulse :type "Vector Structure") (Hit :type "HitResult Structure (by ref)"))
  (`NiagaraFunctionLibrary.SpawnSystemAtLocation` null (`self.K2_GetActorLocation`))
  (`GameplayStatics.PlaySound2D` (`self.BulletExplodeSound`) 1.0 1.0 0.0 null null)
  (`self.K2_DestroyActor`))

(fn `UserConstructionScript`
  (`self.SetLifeSpan` (`self.LifespanVal`)))